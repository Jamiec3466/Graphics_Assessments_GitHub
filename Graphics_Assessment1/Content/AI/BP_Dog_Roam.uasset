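; Dog actor that wanders the level and plays an animation when the player interacts with it.
; From BeginPlay, DogWalk issues an AI move to a random reachable point, then calls itself after a short delay from the immediate output, without waiting for arrival.
; Box overlap toggles player input, so pressing E nearby plays the dog animation once.
; The RandomRoam function is an empty stub.
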(event `self.Box.OnComponentBeginOverlap`
  (params (OverlappedComponent :type "PrimitiveComponent Object Reference") (OtherActor :type "Actor Object Reference") (OtherComp :type "PrimitiveComponent Object Reference") (OtherBodyIndex :type Integer) (bFromSweep :type Boolean) (SweepResult :type "HitResult Structure (by ref)"))
  ; Checking if the player is within the collision detection of the door object
  (`self.EnableInput` (`GameplayStatics.GetPlayerController` 0)))

(event `self.Box.OnComponentEndOverlap`
  (params (OverlappedComponent :type "PrimitiveComponent Object Reference") (OtherActor :type "Actor Object Reference") (OtherComp :type "PrimitiveComponent Object Reference") (OtherBodyIndex :type Integer))
  ; Checking if the player is within the collision detection of the door object
  (`self.DisableInput` (`GameplayStatics.GetPlayerController` 0)))

(event `self.ReceiveBeginPlay`
  (`self.DogWalk`))

(event `DogWalk`
  (`|AIMoveTo` self (`NavigationSystemV1.K2_GetRandomReachablePointInRadius` (`self.K2_GetActorLocation`) 25000.0 null null) null
    (:`then`
      (`KismetSystemLibrary.Delay` 1.0)
      (`self.DogWalk`))))

(event `Key|E`
  (params (Key :type "Key Structure"))
  ; Checking input
  (:`Pressed`
    (`SkeletalMeshComponent.PlayAnimation` (`self.Mesh`) "/Game/AI/Dog_Anim.Dog_Anim" false)))

(fn `random roam`)

(fn `UserConstructionScript`)