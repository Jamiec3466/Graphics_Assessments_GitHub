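; BP_periscope is an interactable periscope that switches the player's view to another view target, BEV, while E is held.
; An overlap box enables and disables the actor's input as something enters or leaves it, without checking which actor overlapped.
; Pressing E blends the camera to BEV, and releasing it blends back to the owner of the third-person character's follow camera, cached at BeginPlay.
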(event `self.Box.OnComponentBeginOverlap`
  (params (OverlappedComponent :type "PrimitiveComponent Object Reference") (OtherActor :type "Actor Object Reference") (OtherComp :type "PrimitiveComponent Object Reference") (OtherBodyIndex :type Integer) (bFromSweep :type Boolean) (SweepResult :type "HitResult Structure (by ref)"))
  ; Checking if the player is within the collision detection of the object
  (`self.EnableInput` (`GameplayStatics.GetPlayerController` 0)))

(event `self.Box.OnComponentEndOverlap`
  (params (OverlappedComponent :type "PrimitiveComponent Object Reference") (OtherActor :type "Actor Object Reference") (OtherComp :type "PrimitiveComponent Object Reference") (OtherBodyIndex :type Integer))
  ; Checking if the player is within the collision detection of the object
  (`self.DisableInput` (`GameplayStatics.GetPlayerController` 0)))

(event `self.ReceiveBeginPlay`
  (bind _returnvalue (`GameplayStatics.GetActorOfClass` "/Game/ThirdPerson/Blueprints/BP_ThirdPersonCharacter.BP_ThirdPersonCharacter_C"))
  (set `self.Follow` (`/Game/ThirdPerson/Blueprints/BP_ThirdPersonCharacter.FollowCamera` _returnvalue)))

(event `Key|E`
  (params (Key :type "Key Structure"))
  (:`Pressed`
    (`PlayerController.SetViewTargetWithBlend` (`GameplayStatics.GetPlayerController` 0) (`self.BEV`) 0.3 "VTBlend_Linear" 0.0 false))
  (:`Released`
    (`PlayerController.SetViewTargetWithBlend` (`GameplayStatics.GetPlayerController` 0) (`ActorComponent.GetOwner` (`self.Follow`)) 0.3 "VTBlend_Linear" 0.0 false)))

(fn `UserConstructionScript`)