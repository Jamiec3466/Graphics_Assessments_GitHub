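; BP_Switch is a light switch actor that lets the player toggle three spotlights while standing inside its overlap area.
; Beginning an overlap enables input for player controller 0 and ending it disables input, without checking which actor overlapped.
; Pressing E flips the LightOn flag and sets the intensity of all three referenced spotlights to either full brightness or zero.
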(event `self.ReceiveActorBeginOverlap`
  (params (OtherActor :type "Actor Object Reference"))
  ; Checking if the player is within the collision detection of the lightswitch object
  (`self.EnableInput` (`GameplayStatics.GetPlayerController` 0)))

(event `self.ReceiveActorEndOverlap`
  (params (OtherActor :type "Actor Object Reference"))
  ; Checking if the player is within the collision detection of the lightswitch object
  (`self.DisableInput` (`GameplayStatics.GetPlayerController` 0)))

(event `Key|E`
  (params (Key :type "Key Structure"))
  (bind _spotlightcomponent (`SpotLight.SpotLightComponent` (`self.Light3`)))
  (bind _spotlightcomponent_2 (`SpotLight.SpotLightComponent` (`self.spotlight`)))
  (bind _spotlightcomponent_3 (`SpotLight.SpotLightComponent` (`self.Light2`)))
  (:`Pressed`
    (if (not (`self.LightOn`))
      (set `self.LightOn` true)
      (`LightComponent.SetIntensity` _spotlightcomponent_2 1000.0)
      (`LightComponent.SetIntensity` _spotlightcomponent_3 1000.0)
      (`LightComponent.SetIntensity` _spotlightcomponent 1000.0)
      (else
        (set `self.LightOn` false)
        (`LightComponent.SetIntensity` _spotlightcomponent_2 0.0)
        (`LightComponent.SetIntensity` _spotlightcomponent_3 0.0)
        (`LightComponent.SetIntensity` _spotlightcomponent 0.0)))))

(fn `UserConstructionScript`)